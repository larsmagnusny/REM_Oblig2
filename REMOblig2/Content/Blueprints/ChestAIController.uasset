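; AI controller for a chest pawn that either follows a player or travels to a slot.
; On BeginPlay it runs a behavior tree and caches the pawn's ChestController component.
; Each tick it copies that component's state to the blackboard: Target is the followed player, the slot or empty, and while following, AwayFromTarget is a horizontal offset away from the player.
; Within range of the slot, it ends the trip and tells the component to snap in.
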(event `self.ReceiveBeginPlay`
  (`self.RunBehaviorTree` "/Game/Blueprints/AI_BT.AI_BT")
  (set `self.ChestController` (`self.GetComponentByClass` (`self.K2_GetPawn`) "/Script/REMOblig2.ChestController")))

(event `self.ReceiveTick`
  (params (DeltaSeconds :type "Float (single-precision)"))
  (bind _chestcontroller (`self.ChestController`))
  (bind _returnvalue (`self.GetComponentByClass` (`self.K2_GetPawn`) "/Script/REMOblig2.ChestController"))
  (bind _returnvalue_2 (`AIBlueprintHelperLibrary.GetBlackboard` self))
  (bind _returnvalue_3 (`self.K2_GetActorLocation` (`ActorComponent.GetOwner` _returnvalue)))
  (if (`ChestController.FollowingPlayer` _returnvalue)
    (`BlackboardComponent.SetValueAsObject` _returnvalue_2 "Target" (`ChestController.PlayerToFollow` _returnvalue))
    (`BlackboardComponent.SetValueAsVector` _returnvalue_2 "AwayFromTarget" (+ _returnvalue_3 (`KismetMathLibrary.Conv_Vector2DToVector` (* (`KismetMathLibrary.Normal2D` (- (`KismetMathLibrary.Conv_VectorToVector2D` _returnvalue_3) (`KismetMathLibrary.Conv_VectorToVector2D` (`self.K2_GetActorLocation` (`ChestController.PlayerToFollow` _returnvalue))))) 100.0))))
    (elif (`ChestController.GoToSlot` _returnvalue)
      (bind _returnvalue_4 (`ChestController.SlotToGoTo` _returnvalue))
      (`BlackboardComponent.SetValueAsObject` _returnvalue_2 "Target" _returnvalue_4)
      (if (< (`self.GetDistanceTo` (`self.K2_GetPawn`) _returnvalue_4) 100.0)
        (set `ChestController.GoToSlot` false _chestcontroller)
        (`ChestController.SnapToSlot` _chestcontroller))
      (else
        (`BlackboardComponent.SetValueAsObject` _returnvalue_2 "Target" null)))))

(fn `UserConstructionScript`)