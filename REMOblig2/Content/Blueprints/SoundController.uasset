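; SoundController is a component that keeps its owner's AudioComponent volume in step with the main menu fade and master volume.
; On BeginPlay it caches the HUD's MainMenu widget, the owner's AudioComponent and the game instance.
; Each Tick it applies (1 − CurFade) × MasterVolume when that value changes.
; Stopped audio restarts once the last volume is non-zero; at zero, it only refreshes the stored volume.
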(event `self.ReceiveBeginPlay`
  (bind _asrem_hud (cast `REM_Hud` (`PlayerController.GetHUD` (`GameplayStatics.GetPlayerController` 0))))
  (bind _asmain_menu (cast `/Game/UI/MainMenu` (`REM_Hud.MainMenuWidget` _asrem_hud)))
  (set `self.MainMenu` _asmain_menu)
  (set `self.AudioComponent` (`Actor.GetComponentByClass` (`self.GetOwner`) "/Script/Engine.AudioComponent"))
  (bind _asrem_game_instance (cast `REM_GameInstance` (`GameplayStatics.GetGameInstance`)))
  (set `self.Gameinstance` _asrem_game_instance))

(event `self.ReceiveTick`
  (params (DeltaSeconds :type "Float (single-precision)"))
  (bind _audiocomponent (`self.AudioComponent`))
  (bind _returnvalue (* (- 1.0 (`/Game/UI/MainMenu.CurFade` (`self.MainMenu`))) (`REM_GameInstance.MasterVolume` (`self.Gameinstance`))))
  (if (`AudioComponent.IsPlaying` _audiocomponent)
    (if (not (== (`self.LastVolume`) _returnvalue)) :!label _label
      (`AudioComponent.AdjustVolume` (`self.AudioComponent`) 0.0 _returnvalue)
      (set `self.LastVolume` _returnvalue))
    (elif (== (`self.LastVolume`) 0.0)
      (set `self.LastVolume` _returnvalue)
      (else
        (`AudioComponent.Play` _audiocomponent 0.0)
        (goto _label)))))