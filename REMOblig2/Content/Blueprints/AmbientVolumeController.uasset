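; An actor component that ties its owner's ambient audio volume to the HUD's current opacity and the game's master volume.
; On BeginPlay it caches the REM HUD and game instance.
; Each Tick it restarts the owner's AudioComponent if stopped and multiplies inverse HUD opacity by master volume, so sound fades as opacity rises.
; It floors the result at zero and applies it only when it differs from the last value.
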(event `self.ReceiveBeginPlay`
  (bind _asrem_hud (cast `REM_Hud` (`PlayerController.GetHUD` (`GameplayStatics.GetPlayerController` 0))))
  (set `self.HudReference` _asrem_hud)
  (bind _asrem_game_instance (cast `REM_GameInstance` (`GameplayStatics.GetGameInstance`)))
  (set `self.GameInstance` _asrem_game_instance))

(event `self.ReceiveTick`
  (params (DeltaSeconds :type "Float (single-precision)"))
  (bind _returnvalue (`Actor.GetComponentByClass` (`self.GetOwner`) "/Script/Engine.AudioComponent"))
  (bind _returnvalue_2 (* (- 1.0 (`REM_Hud.CurrentOpacity` (`self.HudReference`))) (`REM_GameInstance.MasterVolume` (`self.GameInstance`))))
  (if (not (`AudioComponent.IsPlaying` _returnvalue))
    (`AudioComponent.Play` _returnvalue 0.0))
  (set `self.Volume` _returnvalue_2)
  (if (!= _returnvalue_2 (`self.LastVolume`))
    (if (< _returnvalue_2 0.0)
      (set `self.Volume` 0.0))
    (`AudioComponent.SetVolumeMultiplier` _returnvalue (`self.Volume`))
    (set `self.LastVolume` (`self.Volume`))))